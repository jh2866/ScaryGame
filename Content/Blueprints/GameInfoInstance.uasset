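; GameInfoInstance, likely a Game Instance, provides events that display the main, options and credits menus.
; The main and options widgets are created for player 0 on first use, cached in variables and re-added to the viewport on later calls.
; The credits widget is created anew on every call, and only the main menu event turns on the mouse cursor.
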(event Custom|ShowMainMenu
  (bind _returnvalue (Game|GetPlayerController 0))
  ;[1 1 1] Show Main Menu
  (Utilities|IsValid (Variables|Default|GetMainMenuWB)
    (:Is%20Valid
      _)
    (:Is%20Not%20Valid
      (bind _returnvalue_2 (UserInterface|CreateWidget "/Game/Maps/MainMenu/MainMenuUI.MainMenuUI_C" _returnvalue))
      (Variables|Default|SetMainMenuWB _returnvalue_2)))
  (UserInterface|Viewport|AddtoViewport (Variables|Default|GetMainMenuWB) 0)
  (Variables|/Script/Engine.PlayerController|SetbShowMouseCursor _returnvalue true))

(event Custom|ShowOptionsMenu
  ;[1 1 1] Show Options Menu
  (Utilities|IsValid (Variables|Default|GetOptionsMenuWB)
    (:Is%20Valid
      _)
    (:Is%20Not%20Valid
      (bind _returnvalue (UserInterface|CreateWidget "/Game/Maps/MainMenu/OptionsMenu.OptionsMenu_C" (Game|GetPlayerController 0)))
      (Variables|Default|SetOptionsMenuWB _returnvalue)))
  (UserInterface|Viewport|AddtoViewport (Variables|Default|GetOptionsMenuWB) 0))

(event Custom|ShowCreditsMenu
  ;[1 1 1] Show Credits Menu
  (bind _returnvalue (UserInterface|CreateWidget "/Game/Maps/MainMenu/CreditsMenu.CreditsMenu_C" (Game|GetPlayerController 0)))
  (UserInterface|Viewport|AddtoViewport _returnvalue 0))